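; Portal audio actor that hands ambience between two areas, A and B, as the first-person character crosses between them.
; Entering either trigger fades in that area's 2D ambience on the character.
; Leaving one trigger while inside both fades out its 2D sound, fades in its 3D emitter and cuts the other emitter.
; SET_AMB parameters select each side's sound, and the B emitter starts playing on BeginPlay.
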(event `self.ReceiveBeginPlay`
  ;[0.7899 1 0.5518] [SD] Ambience System
  (`AudioParameterControllerInterface.SetIntParameter` (`self.Audio_3D_AMB_A`) "SET_AMB" (`self.AudioAMB_A`))
  (`AudioParameterControllerInterface.SetIntParameter` (`self.Audio_3D_AMB_B`) "SET_AMB" (`self.AudioAMB_B`))
  (`AudioComponent.Play` (`self.Audio_3D_AMB_B`) 0.5))

(event `self.Trigger_A.OnComponentBeginOverlap`
  (params (OverlappedComponent :type "PrimitiveComponent Object Reference") (OtherActor :type "Actor Object Reference") (OtherComp :type "PrimitiveComponent Object Reference") (OtherBodyIndex :type Integer) (bFromSweep :type Boolean) (SweepResult :type "HitResult Structure (by ref)"))
  ;[0.7899 1 0.5518] [SD] Ambience System
  (if (not (`self.InsideA`))
    (bind _asfirst_person_character (cast `/Game/Blueprints/Player/FirstPersonCharacter` OtherActor))
    (set `self.InsideA` true)
    (bind _audio_2d_amb_a (`/Game/Blueprints/Player/FirstPersonCharacter.Audio_2D_AMB_A` _asfirst_person_character))
    (`AudioParameterControllerInterface.SetIntParameter` _audio_2d_amb_a "SET_AMB" (`self.AudioAMB_A`))
    (`AudioComponent.FadeIn` _audio_2d_amb_a 0.5 1.0 0.0 "Linear")
    (if (`self.InsideB`)
      (set `self.InsideBoth` true))))

(event `self.Trigger_B.OnComponentBeginOverlap`
  (params (OverlappedComponent :type "PrimitiveComponent Object Reference") (OtherActor :type "Actor Object Reference") (OtherComp :type "PrimitiveComponent Object Reference") (OtherBodyIndex :type Integer) (bFromSweep :type Boolean) (SweepResult :type "HitResult Structure (by ref)"))
  ;[0.7899 1 0.5518] [SD] Ambience System
  (if (not (`self.InsideB`))
    (bind _asfirst_person_character (cast `/Game/Blueprints/Player/FirstPersonCharacter` OtherActor))
    (set `self.InsideB` true)
    (bind _audio_2d_amb_b (`/Game/Blueprints/Player/FirstPersonCharacter.Audio_2D_AMB_B` _asfirst_person_character))
    (`AudioParameterControllerInterface.SetIntParameter` _audio_2d_amb_b "SET_AMB" (`self.AudioAMB_B`))
    (`AudioComponent.FadeIn` _audio_2d_amb_b 0.5 1.0 0.0 "Linear")
    (if (`self.InsideA`)
      (set `self.InsideBoth` true))))

(event `self.Trigger_A.OnComponentEndOverlap`
  (params (OverlappedComponent :type "PrimitiveComponent Object Reference") (OtherActor :type "Actor Object Reference") (OtherComp :type "PrimitiveComponent Object Reference") (OtherBodyIndex :type Integer))
  ;[0.7899 1 0.5518] [SD] Ambience System
  (if (`self.InsideBoth`)
    (bind _asfirst_person_character (cast `/Game/Blueprints/Player/FirstPersonCharacter` OtherActor))
    (set `self.InsideA` false)
    (`AudioComponent.FadeOut` (`/Game/Blueprints/Player/FirstPersonCharacter.Audio_2D_AMB_A` _asfirst_person_character) 0.5 0.0 "Linear")
    (`AudioComponent.FadeIn` (`self.Audio_3D_AMB_A`) 0.5 1.0 0.0 "Linear")
    (`AudioComponent.FadeOut` (`self.Audio_3D_AMB_B`) 0.0 0.0 "Linear")
    (set `self.InsideBoth` false)))

(event `self.Trigger_B.OnComponentEndOverlap`
  (params (OverlappedComponent :type "PrimitiveComponent Object Reference") (OtherActor :type "Actor Object Reference") (OtherComp :type "PrimitiveComponent Object Reference") (OtherBodyIndex :type Integer))
  ;[0.7899 1 0.5518] [SD] Ambience System
  (if (`self.InsideBoth`)
    (bind _asfirst_person_character (cast `/Game/Blueprints/Player/FirstPersonCharacter` OtherActor))
    (set `self.InsideB` false)
    (`AudioComponent.FadeOut` (`/Game/Blueprints/Player/FirstPersonCharacter.Audio_2D_AMB_B` _asfirst_person_character) 0.5 0.0 "Linear")
    (`AudioComponent.FadeIn` (`self.Audio_3D_AMB_B`) 0.5 1.0 0.0 "Linear")
    (`AudioComponent.FadeOut` (`self.Audio_3D_AMB_A`) 0.0 0.0 "Linear")
    (set `self.InsideBoth` false)))

(fn `UserConstructionScript`)