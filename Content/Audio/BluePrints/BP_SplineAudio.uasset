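; Blueprint actor that makes an ambient sound follow the player along a spline, such as for a long or shaped audio source.
; On BeginPlay it starts the Audio component at a random offset within the sound's duration.
; A self-calling MoveAudio loop moves the component every 0.05 seconds to the spline point closest to the player character, raised slightly in Z.
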(event `self.ReceiveBeginPlay`
  (bind _audio (`self.Audio`))
  ;[0.7899 1 0.5518] [SD]
  (`AudioComponent.Play` _audio (`KismetMathLibrary.RandomFloatInRange` 0.0 (`SoundBase.Duration` (`AudioComponent.Sound` _audio))))
  (`self.Move Audio`))

(event `Move Audio`
  (bind (_returnvalue_x _returnvalue_y _returnvalue_z) (`KismetMathLibrary.BreakVector` (`SplineComponent.FindLocationClosestToWorldLocation` (`self.Spline`) (`self.K2_GetActorLocation` (`GameplayStatics.GetPlayerCharacter` 0)) "World")))
  ;[0.7899 1 0.5518] [SD]
  (`SceneComponent.K2_SetWorldLocation` (`self.Audio`) (`KismetMathLibrary.MakeVector` _returnvalue_x _returnvalue_y (+ _returnvalue_z 50.0)) false false)
  (`KismetSystemLibrary.Delay` 0.05)
  (`self.Move Audio`))

(fn `UserConstructionScript`)